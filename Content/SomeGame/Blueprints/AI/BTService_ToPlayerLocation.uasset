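; Behavior tree service that, despite its ToPlayerLocation name, feeds the AI the location of the TriggerGate actor.
; On AI activation it finds that actor by class and writes its location to the selected vector blackboard key, with no tick updates.
; A disconnected branch would instead write the player pawn's nav location, or a random nearby navigable point when that pawn is not controlled.
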(event `self.ReceiveActivationAI`
  (params (OwnerController :type "AIController Object Reference") (ControlledPawn :type "Pawn Object Reference"))
  (bind _returnvalue (`GameplayStatics.GetActorOfClass` "/Script/task16.TriggerGate"))
  (`BTFunctionLibrary.SetBlackboardValueAsVector` (`self.BlackboardKey`) (`Actor.K2_GetActorLocation` _returnvalue)))