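; Behavior tree service that writes a target location into a Blackboard vector key for an AI.
; On activation it sets the key to a fixed, hard-coded world position.
; An unconnected branch, which never runs, would write the player pawn's nav agent location when that pawn is controlled, or a random navigable point otherwise.
; Despite the asset's name, the live logic does not track the player.
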(event `self.ReceiveActivationAI`
  (params (OwnerController :type "AIController Object Reference") (ControlledPawn :type "Pawn Object Reference"))
  (`BTFunctionLibrary.SetBlackboardValueAsVector` (`self.BlackboardKey`) (`KismetMathLibrary.MakeVector` 640.0 4000.0 23.0)))